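; BP_SpherePosition is an actor that moves a sphere and reports its position to a Niagara effect.
; Each Tick shifts the Sphere component by a fixed step along world X, without sweep and independent of frame time.
; It then writes the sphere's world location to the Niagara component's SpherePosition variable, so the particle system can follow the moving sphere.
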(event EventBeginPlay)

(event Collision|EventActorBeginOverlap
  (params (OtherActor :type Actor%20Object%20Reference)))

(event EventTick
  (params (DeltaSeconds :type Float%20%28single-precision%29))
  (bind _sphere (Variables|Default|GetSphere))
  (Transformation|SetWorldLocation _sphere (+ (Transformation|GetWorldLocation _sphere) "5.000000,0.000000,0.000000") false false)
  (Class|NiagaraComponent|SetVariablePosition (Variables|Default|GetNiagara) "SpherePosition" (Transformation|GetWorldLocation (Variables|Default|GetSphere))))

(fn ConstructionScript)